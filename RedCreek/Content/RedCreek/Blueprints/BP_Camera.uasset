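; BP_Camera is the player's point-and-click hub, handling mouse interaction, HUD and pause menu.
; On BeginPlay it shows the cursor, adds the HUD and creates the PauseMenu widget.
; Left and right clicks trace under the cursor and message hit actors implementing BPI_Mouse, while OnHover and OnRelease set or clear HoverText.
; Pause freezes the game and swaps HUD for menu; UnPause only re-adds the HUD.
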(event `self.ReceiveBeginPlay`
  (bind _returnvalue (`GameplayStatics.GetPlayerController` 0))
  (set `PlayerController.bShowMouseCursor` true _returnvalue)
  (set `PlayerController.bEnableMouseOverEvents` true _returnvalue)
  (bind _returnvalue_2 (`|CreateWidget` "/Game/RedCreek/Blueprints/UserInterface/UI.UI_C"))
  (bind _output_get (set `self.HUD` _returnvalue_2))
  (`UserWidget.AddToViewport` _output_get 0)
  (bind _returnvalue_3 (`|CreateWidget` "/Game/RedCreek/Blueprints/UserInterface/PauseMenu.PauseMenu_C"))
  (set `self.PauseMenu` _returnvalue_3))

(event `/Game/RedCreek/Blueprints/BPI_Mouse.OnHover`
  (params (DisplayText :type String))
  (set `self.HoverText` DisplayText))

(event `/Game/RedCreek/Blueprints/BPI_Mouse.OnRelease`
  (set `self.HoverText` ""))

(event `InputAction|RightClick`
  (params (Key :type "Key Structure" :default "AnyKey"))
  (bind (_bblockinghit _binitialoverlap _time _location _impactpoint _normal _impactnormal _physmat _hitactor) (`GameplayStatics.BreakHitResult` (`PlayerController.GetHitResultUnderCursorByChannel` (`GameplayStatics.GetPlayerController` 0) "TraceTypeQuery1" true)))
  (:`Pressed`
    (if (`KismetSystemLibrary.DoesImplementInterface` _hitactor "/Game/RedCreek/Blueprints/BPI_Mouse.BPI_Mouse_C")
      (message `/Game/RedCreek/Blueprints/BPI_Mouse.BPI_OnRightClick` _hitactor))))

(event `InputAction|LeftClick`
  (params (Key :type "Key Structure" :default "AnyKey"))
  (bind (_bblockinghit _binitialoverlap _time _location _impactpoint _normal _impactnormal _physmat _hitactor) (`GameplayStatics.BreakHitResult` (`PlayerController.GetHitResultUnderCursorByChannel` (`GameplayStatics.GetPlayerController` 0) "TraceTypeQuery1" true)))
  (:`Pressed`
    (if (`KismetSystemLibrary.DoesImplementInterface` _hitactor "/Game/RedCreek/Blueprints/BPI_Mouse.BPI_Mouse_C")
      (message `/Game/RedCreek/Blueprints/BPI_Mouse.BPI_OnLeftClick` _hitactor))))

(event `InputAction|Pause`
  (params (Key :type "Key Structure" :default "AnyKey"))
  (:`Pressed`
    (`GameplayStatics.SetGamePaused` true)
    (`Widget.RemoveFromParent` (`self.HUD`))
    (`UserWidget.AddToViewport` (`self.PauseMenu`) 0)))

(event `UnPause`
  (`UserWidget.AddToViewport` (`self.HUD`) 0))

(fn `UserConstructionScript`)